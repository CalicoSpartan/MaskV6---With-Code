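; Player controller for a team-based FPS that creates and updates the player's HUD, team score bars and scoreboard.
; UI events add the game and score widgets, register the game UI on the GameState, and set both score bars' percentages and team colors.
; The scoreboard is built hidden from GameState teams and their player states, and shown while Tab is held.
; Stat updates rebind existing rows to player states by index instead of rebuilding them.
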(event Custom|UpdateScore
  (bind _scoreui (Variables|Default|GetScoreUI))
  (bind _myscore (Variables|/Game/UI/ScoreUI.ScoreUI_C|GetMyScore _scoreui))
  (bind _enemyscore (Variables|/Game/UI/ScoreUI.ScoreUI_C|GetEnemyScore _scoreui))
  ;[1 1 1] ScoreUI
  (Utilities|IsValid (Variables|Default|GetScoreUI)
    (:Is%20Valid
      (Progress|SetPercent _myscore (Variables|Default|GetTeamScorePercent))
      (Progress|SetPercent _enemyscore (Variables|Default|GetRivalScorePercent))
      (bind _asbp_fpsplayer_state (Utilities|Casting|CastToBP_FPSPlayerState (Variables|Default|GetPlayerState)))
      (Utilities|IsValid (Variables|/Script/FPSProject.FPSPlayerState|GetTeam _asbp_fpsplayer_state)
        (:Is%20Valid
          (Class|ProgressBar|SetFillColorandOpacity _myscore (Math|Conversions|ToLinearColor(Color) (Variables|/Script/FPSProject.BaseTeam|GetTeamColor (Variables|/Script/FPSProject.FPSPlayerState|GetTeam _asbp_fpsplayer_state))))
          (Utilities|IsValid (Variables|/Script/FPSProject.FPSPlayerState|GetRivalTeam _asbp_fpsplayer_state)
            (:Is%20Valid
              (Class|ProgressBar|SetFillColorandOpacity _enemyscore (Math|Conversions|ToLinearColor(Color) (Variables|/Script/FPSProject.BaseTeam|GetTeamColor (Variables|/Script/FPSProject.FPSPlayerState|GetRivalTeam _asbp_fpsplayer_state)))))))))))

(event Custom|RemoveScoreBoard
  (bind _scoreboardui (Variables|Default|GetScoreBoardUI))
  (Utilities|IsValid _scoreboardui
    (:Is%20Valid
      (Widget|SetVisibility _scoreboardui "Hidden"))))

(event Custom|AddGameUIToClient
  ;[1 1 1] GameUI
  (Utilities|IsValid (Variables|Default|GetInGameUI)
    (:Is%20Not%20Valid
      (bind _returnvalue (UserInterface|CreateWidget "/Game/UI/InGameUI.InGameUI_C"))
      (bind _output_get (Variables|Default|SetInGameUI _returnvalue))
      (bind _asbp_game_state (Utilities|Casting|CastToBP_GameState (Game|GetGameState)))
      (Variables|/Game/Blueprints/BP_GameState.BP_GameState_C|SetUI _asbp_game_state _returnvalue)
      (UserInterface|Viewport|AddtoViewport _output_get 0)
      (bind _returnvalue_2 (UserInterface|CreateWidget "/Game/UI/ScoreUI.ScoreUI_C"))
      (bind _output_get_2 (Variables|Default|SetScoreUI _returnvalue_2))
      (UserInterface|Viewport|AddtoViewport _output_get_2 1))))

(event Custom|UpdatePlayerStats
  (bind _scoreboardui (Variables|Default|GetScoreBoardUI))
  (bind _verticalscorebox (Variables|/Game/UI/ScoreBoardUI.ScoreBoardUI_C|GetVerticalScoreBox _scoreboardui))
  ;[1 1 1] UpdateScoreBoard
  (Utilities|IsValid _scoreboardui
    (:Is%20Valid
      (Variables|Default|SetTeamIterator 0)
      (while (< (Variables|Default|GetTeamIterator) (Class|PanelWidget|GetChildrenCount _verticalscorebox))
        (bind _asteam_score_board (Utilities|Casting|CastToTeamScoreBoard (Class|PanelWidget|GetChildat _verticalscorebox (Variables|Default|GetTeamIterator))))
        (Variables|Default|SetPlayerStateIterator 0)
        (while (< (Variables|Default|GetPlayerStateIterator) (Class|PanelWidget|GetChildrenCount (Variables|/Game/UI/TeamScoreBoard.TeamScoreBoard_C|GetAddTeamsToThisBox _asteam_score_board)))
          (bind _asplayer_stats (Utilities|Casting|CastToPlayerStats (Class|PanelWidget|GetChildat (Variables|/Game/UI/TeamScoreBoard.TeamScoreBoard_C|GetAddTeamsToThisBox _asteam_score_board) (Variables|Default|GetPlayerStateIterator))))
          (bind _asbp_fpsplayer_state (Utilities|Casting|CastToBP_FPSPlayerState (Utilities|Array|Get(acopy) (Variables|/Script/FPSProject.BaseTeam|GetTeamPlayerStates (Variables|/Game/UI/TeamScoreBoard.TeamScoreBoard_C|GetTeamReference _asteam_score_board)) (Variables|Default|GetPlayerStateIterator))))
          (Default|SetReferencedPlayer _asplayer_stats _asbp_fpsplayer_state)
          (Math|Integer|IncrementInt (Variables|Default|GetPlayerStateIterator)))
        (Math|Integer|IncrementInt (Variables|Default|GetTeamIterator))))))

(event Custom|AddScoreBoardToClient
  ;[1 1 1] base scoreboard
  (Utilities|IsValid (Variables|Default|GetScoreBoardUI)
    (:Is%20Not%20Valid
      (bind _returnvalue (UserInterface|CreateWidget "/Game/UI/ScoreBoardUI.ScoreBoardUI_C"))
      (Variables|Default|SetScoreBoardUI _returnvalue)
      (bind _asbp_game_state (Utilities|Casting|CastToBP_GameState (Game|GetGameState)))
      (for _array_element (Variables|/Script/FPSProject.FPSGameState|GetTeams _asbp_game_state)
        (bind _asbp_base_team (Utilities|Casting|CastToBP_BaseTeam _array_element))
        (bind _returnvalue_2 (UserInterface|CreateWidget "/Game/UI/TeamScoreBoard.TeamScoreBoard_C" 0 _asbp_base_team))
        (Class|VerticalBox|AddChildtoVerticalBox (Variables|/Game/UI/ScoreBoardUI.ScoreBoardUI_C|GetVerticalScoreBox (Variables|Default|GetScoreBoardUI)) _returnvalue_2)
        (for _array_element_2 (Variables|/Script/FPSProject.BaseTeam|GetTeamPlayerStates _asbp_base_team)
          (bind _asbp_fpsplayer_state (Utilities|Casting|CastToBP_FPSPlayerState _array_element_2))
          (bind _returnvalue_3 (UserInterface|CreateWidget "/Game/UI/PlayerStats.PlayerStats_C" 0 0))
          (Default|SetReferencedPlayer _returnvalue_3 _asbp_fpsplayer_state)
          (Appearance|SetColorandOpacity _returnvalue_3 (Math|Conversions|ToLinearColor(Color) (Variables|/Script/FPSProject.BaseTeam|GetTeamColor _asbp_base_team)) :!class /Script/UMG.UserWidget)
          (Class|VerticalBox|AddChildtoVerticalBox (Variables|/Game/UI/TeamScoreBoard.TeamScoreBoard_C|GetAddTeamsToThisBox _returnvalue_2) _returnvalue_3)))
      (Widget|SetVisibility (Variables|Default|GetScoreBoardUI) "Hidden")
      (UserInterface|Viewport|AddtoViewport (Variables|Default|GetScoreBoardUI) 0))))

(event Custom|ShowScoreBoard
  (bind _scoreboardui (Variables|Default|GetScoreBoardUI))
  (Utilities|IsValid _scoreboardui
    (:Is%20Valid
      (Widget|SetVisibility _scoreboardui "Visible"))))

(event EventTriggerAddAliveUIBlueprint
  ;[1 1 1] GameUI
  (CallFunction|AddGameUItoClient))

(event EventUpdateScoreBoardUIBlueprint
  ;[1 1 1] UpdateScoreBoard
  (CallFunction|UpdatePlayerStats))

(event EventUpdateScoreUIBlueprint
  ;[1 1 1] ScoreUI
  (CallFunction|UpdateScore))

(event EventAddScoreBoardUIBlueprint
  ;[1 1 1] base scoreboard
  (CallFunction|AddScoreBoardtoClient))

(event Input|KeyboardEvents|Tab
  (params (Key :type Key%20Structure))
  (:Pressed
    (CallFunction|ShowScoreBoard))
  (:Released
    (CallFunction|RemoveScoreBoard)))

(fn ConstructionScript)