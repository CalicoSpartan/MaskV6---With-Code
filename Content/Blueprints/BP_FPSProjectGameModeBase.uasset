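; Game mode Blueprint that drives the game countdown display through BP_GameState.
; Each Tick, while GameCountdownTimer is valid, it passes the timer's remaining time to the game state's ShowGameCountdown.
; Once the timer is no longer valid and the state is Playing, it calls StopShowingCountdown, using the HasTurnedOffCountdown flag to do so only once.
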(event EventTick
  (params (DeltaSeconds :type Float%20%28single-precision%29))
  (bind _gamecountdowntimer (Variables|Default|GetGameCountdownTimer))
  ;[1 1 1] CountdownTimer
  (if (Utilities|Time|IsValidTimerHandle _gamecountdowntimer)
    (bind _asbp_game_state (Utilities|Casting|CastToBP_GameState (Game|GetGameState)))
    (Default|ShowGameCountdown _asbp_game_state (Utilities|Time|GetTimerRemainingTimebyHandle _gamecountdowntimer))
    (else
      (bind _asbp_game_state_2 (Utilities|Casting|CastToBP_GameState (Game|GetGameState)))
      (if (Utilities|Enum|Equal(Enum) (Class|FPSGameState|GetCurrentState _asbp_game_state_2) "EPlaying")
        (if (not (Variables|Default|GetHasTurnedOffCountdown))
          (bind _asbp_game_state_3 (Utilities|Casting|CastToBP_GameState (Game|GetGameState)))
          (Default|StopShowingCountdown _asbp_game_state_3)
          (Variables|Default|SetHasTurnedOffCountdown true))))))

(fn ConstructionScript)