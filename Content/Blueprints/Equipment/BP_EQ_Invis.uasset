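; Invisibility equipment that drives a cloak material effect on the BP_FPSCharacter it is attached to.
; On Applied, the server registers it as the character's InvisibilityAbility and starts the effect using team color.
; While active, Tick feeds UpdateInvisibility an OpaqueValue falling from 1 at rest to 0 at speed, and the server copies lifetime-timer elapsed time to InvisibilityCountdown.
; Destruction restores the original material.
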(event Custom|ServerCreateMAT
  (CallFunction|CreateMAT))

(event Custom|CreateMAT
  (bind _returnvalue (Rendering|Material|CreateDynamicMaterialInstance "/Game/Materials/InvisMAT.InvisMAT" :!class /Script/Engine.KismetMaterialLibrary))
  (Variables|Default|SetInvisMat_INST _returnvalue))

(event EventBeginPlay
  (Networking|SwitchHasAuthority
    (:Authority
      (CallFunction|CreateMAT))
    (:Remote
      (CallFunction|ServerCreateMAT))))

(event Collision|EventActorBeginOverlap
  (params (OtherActor :type Actor%20Object%20Reference)))

(event EventTick
  (params (DeltaSeconds :type Float%20%28single-precision%29))
  (bind _attachedpawn (Variables|Default|GetAttachedPawn))
  (bind _returnvalue (Transformation|GetVelocity _attachedpawn))
  (bind _returnvalue_2 (Math|Vector|VectorLength _returnvalue))
  (bind _returnvalue_3 (/ _returnvalue_2 6e+02))
  (if (Variables|Default|GetbIsActive)
    (Utilities|IsValid _attachedpawn
      (:Is%20Valid
        (bind _asbp_fpscharacter (Utilities|Casting|CastToBP_FPSCharacter _attachedpawn))
        (if (> _returnvalue_3 1.0)
          (bind _output_get (Variables|Default|SetAlphaFade 1.0))
          (Variables|Default|SetOpaqueValue (Math|Float|Lerp 1.0 0.0 _output_get))
          (else
            (bind _output_get_2 (Variables|Default|SetOpaqueValue (Math|Float|Lerp 1.0 0.0 _returnvalue_3)))))
        (bind _returnvalue_4 (Rendering|Material|GetVectorParameterValue (Variables|/Game/Blueprints/BP_FPSCharacter.BP_FPSCharacter_C|GetMyTeamMAT _asbp_fpscharacter) "MyColor" :!class /Script/Engine.MaterialInstanceDynamic))
        (Default|UpdateInvisibility _asbp_fpscharacter 1.06 _output_get_2 (Math|Conversions|ToVector(LinearColor) _returnvalue_4))
        (Networking|SwitchHasAuthority
          (:Authority
            (Variables|/Game/Blueprints/BP_FPSCharacter.BP_FPSCharacter_C|SetInvisibilityCountdown _asbp_fpscharacter (Class|KismetSystemLibrary|GetTimerElapsedTimeHandle (Variables|Default|GetLifeTimeTimer)))))))))

(event EventApplied
  (bind _attachedpawn (Variables|Default|GetAttachedPawn))
  (Networking|SwitchHasAuthority
    (:Authority
      (Utilities|IsValid _attachedpawn
        (:Is%20Valid
          (Development|PrintString "i have a character reference" true true "(R=0.000000,G=0.660000,B=1.000000,A=1.000000)" 5e+02)
          (bind _asbp_fpscharacter (Utilities|Casting|CastToBP_FPSCharacter _attachedpawn))
          (Utilities|IsValid (Variables|/Game/Blueprints/BP_FPSCharacter.BP_FPSCharacter_C|GetMyTeamMAT _asbp_fpscharacter)
            (:Is%20Valid
              (Variables|/Game/Blueprints/BP_FPSCharacter.BP_FPSCharacter_C|SetInvisibilityAbility _asbp_fpscharacter self)
              (bind _returnvalue (Rendering|Material|GetVectorParameterValue (Variables|/Game/Blueprints/BP_FPSCharacter.BP_FPSCharacter_C|GetMyTeamMAT _asbp_fpscharacter) "MyColor" :!class /Script/Engine.MaterialInstanceDynamic))
              (Default|UpdateInvisibility _asbp_fpscharacter 1.06 0.0 (Math|Conversions|ToVector(LinearColor) _returnvalue)))))))))

(event EventDestroyed
  (bind _asbp_fpscharacter (Utilities|Casting|CastToBP_FPSCharacter (Variables|Default|GetAttachedPawn)))
  (Default|SettoOriginalMaterial _asbp_fpscharacter)
  (Actor|DestroyActor))

(fn ConstructionScript)